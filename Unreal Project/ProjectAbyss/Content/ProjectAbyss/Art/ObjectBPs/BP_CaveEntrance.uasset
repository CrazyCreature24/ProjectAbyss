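; BP_CaveEntrance is a level transition actor that moves the player into the ShallowsCave level on overlap.
; Overlapping actors that cast to Divebot are ignored, while others tagged Player trigger the transition.
; The trigger calls the "CaveID" objective in the mission log, then saves all data and the entrance's respawn point through the save/load subsystem before opening the cave level.
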(event `self.ReceiveActorBeginOverlap`
  (params (OtherActor :type "Actor Object Reference"))
  (cast `Divebot` OtherActor
    (:`CastFailed`
      (if (`self.ActorHasTag` OtherActor "Player")
        (`MissionLogSubsystem.CallObjectiveID` (subsystem `MissionLogSubsystem`) "CaveID")
        (`SaveLoadSubsystem.SaveAllData` (subsystem `SaveLoadSubsystem`))
        (`SaveLoadSubsystem.SaveCaveEntrence` (subsystem `SaveLoadSubsystem`) (`self.Respawn point`))
        (`GameplayStatics.OpenLevelBySoftObjectPtr` "/Game/ProjectAbyss/Maps/ShallowsCave.ShallowsCave")))))

(fn `UserConstructionScript`)