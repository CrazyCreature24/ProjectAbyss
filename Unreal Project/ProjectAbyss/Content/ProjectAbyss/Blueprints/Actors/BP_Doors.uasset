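; BP_Doors is a double sliding door actor that opens when an actor tagged Player enters its Box trigger.
; The overlap sets an opening flag, and Tick then calls OpenDoors to slide both leaves apart along local Y by a fixed step each frame.
; A running distance total clears the flag past a limit, so speed depends on frame rate and the doors have no closing logic.
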(event `self.ReceiveTick`
  (params (DeltaSeconds :type "Float (single-precision)"))
  (if (`self.isDoorOpening`)
    (`self.OpenDoors`)))

(event `self.Box.OnComponentBeginOverlap`
  (params (OverlappedComponent :type "PrimitiveComponent Object Reference") (OtherActor :type "Actor Object Reference") (OtherComp :type "PrimitiveComponent Object Reference") (OtherBodyIndex :type Integer) (bFromSweep :type Boolean) (SweepResult :type "HitResult Structure (by ref)"))
  (if (`self.ActorHasTag` OtherActor "Player")
    (set `self.isDoorOpening` true)))

(fn `OpenDoors`
  (`SceneComponent.K2_AddLocalOffset` (`self.RightDoor`) (0.0 2.0 0.0) false false)
  (`SceneComponent.K2_AddLocalOffset` (`self.LeftDoor`) (0.0 -2.0 0.0) false false)
  (bind _output_get (set `self.AmountMoved` (+ (`self.AmountMoved`) 2.0)))
  (if (> _output_get 1200.0)
    (set `self.isDoorOpening` false)))

(fn `UserConstructionScript`)