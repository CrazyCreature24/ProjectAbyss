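; Waypoint trigger actor that shows an objective marker widget when a BP_DiverCharacter enters its Start volume.
; The marker is hidden on BeginPlay, and ToggleWaypoint sets both the enabled flag and widget visibility.
; While enabled, Tick sends the player's distance, truncated to whole meters, to a lazily cached WBP_MarkerDetails.
; The End volume checks for the diver but does nothing, so the marker is never hidden again.
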(event `self.ReceiveBeginPlay`
  (`self.ToggleWaypoint` false))

(event `self.ReceiveTick`
  (params (DeltaSeconds :type "Float (single-precision)"))
  (if (`self.Marker Enabled`)
    (`self.UpdateDistance`)))

(event `self.Start.OnComponentBeginOverlap`
  (params (OverlappedComponent :type "PrimitiveComponent Object Reference") (OtherActor :type "Actor Object Reference") (OtherComp :type "PrimitiveComponent Object Reference") (OtherBodyIndex :type Integer) (bFromSweep :type Boolean) (SweepResult :type "HitResult Structure (by ref)"))
  (if (`GameplayStatics.ObjectIsA` OtherActor "/Game/ProjectAbyss/Blueprints/Actors/Pawns/BP_DiverCharacter.BP_DiverCharacter_C")
    (`self.ToggleWaypoint` true)))

(event `self.End.OnComponentBeginOverlap`
  (params (OverlappedComponent :type "PrimitiveComponent Object Reference") (OtherActor :type "Actor Object Reference") (OtherComp :type "PrimitiveComponent Object Reference") (OtherBodyIndex :type Integer) (bFromSweep :type Boolean) (SweepResult :type "HitResult Structure (by ref)"))
  (if (`GameplayStatics.ObjectIsA` OtherActor "/Game/ProjectAbyss/Blueprints/Actors/Pawns/BP_DiverCharacter.BP_DiverCharacter_C")
    _))

(fn `ToggleWaypoint`
  (params (bNewVisibility :type Boolean))
  (bind _output_get (set `self.Marker Enabled` bNewVisibility))
  (`SceneComponent.SetVisibility` (`self.Widget`) _output_get false))

(fn `UpdateDistance`
  (bind _objective_marker (`self.Objective Marker`)
    (:`then`
      _)
    (:`else`
      (bind _aswbp_marker_details (cast `/Game/ProjectAbyss/Blueprints/Widgets/WBP_MarkerDetails` (`WidgetComponent.GetUserWidgetObject` (`self.Widget`))))
      (set `self.Objective Marker` _aswbp_marker_details)))
  (`/Game/ProjectAbyss/Blueprints/Widgets/WBP_MarkerDetails.Update Distance` _objective_marker (`KismetMathLibrary.FTrunc` (/ (`KismetMathLibrary.Vector_Distance` (`self.K2_GetActorLocation` (`GameplayStatics.GetPlayerCharacter` 0)) (`self.K2_GetActorLocation`)) 100.0))))

(fn `UserConstructionScript`
  (`self.ToggleWaypoint` (`self.Marker Enabled`)))