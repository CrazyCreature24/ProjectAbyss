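; BP_LevelTransition is a trigger actor that saves progress and moves the player to the overworld.
; When an actor tagged Player overlaps it, it saves the divebot, all data and the cave entrance (from Scene) through the SaveLoadSubsystem, then calls LoadOverWorld on MainGameState.
; Mission actor and player state saves are present but disconnected, so they never run.
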(event `self.ReceiveActorBeginOverlap`
  (params (OtherActor :type "Actor Object Reference"))
  (if (`self.ActorHasTag` OtherActor "Player")
    (`SaveLoadSubsystem.SaveDivebot` (subsystem `SaveLoadSubsystem`))
    (`SaveLoadSubsystem.SaveAllData` (subsystem `SaveLoadSubsystem`))
    (`SaveLoadSubsystem.SaveCaveEntrence` (subsystem `SaveLoadSubsystem`) (`self.Scene`))
    (bind _asmain_game_state (cast `MainGameState` (`GameplayStatics.GetGameState`)))
    (`MainGameState.LoadOverWorld` _asmain_game_state)))

(fn `UserConstructionScript`)